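; Simple enemy AI character that wanders, chases sensed characters and can be killed by the player for loot and experience.
; Tick uses a Delay to pace random navmesh moves, while PawnSensing starts a repeating AIMoveTo chase.
; Magic projectile and wooden sword overlaps reduce Health with hit effects, with melee gated by the player's attack state and a short cooldown.
; Death spawns a LootPickup, updates experience and level on ThirdPersonGameMode, then destroys the actor.
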(event OnSeePawn(PawnSensing)
  (params (Pawn :type Pawn%20Object%20Reference))
  (bind _ascharacter (Utilities|Casting|CastToCharacter Pawn))
  (Variables|Default|SetIsMoving true)
  (AI|AIMoveTo self "0, 0, 0" _ascharacter 5.0 false :!label _label
    (:OnSuccess
      _)
    (:OnFail
      _))
  (Utilities|FlowControl|Delay 0.5)
  (goto _label))

(event OnComponentBeginOverlap(CapsuleComponent)
  (params (OverlappedComponent :type Primitive%20Component%20Object%20Reference) (OtherActor :type Actor%20Object%20Reference) (OtherComp :type Primitive%20Component%20Object%20Reference) (OtherBodyIndex :type Integer) (bFromSweep :type Boolean) (SweepResult :type Hit%20Result%20Structure%20%28by%20ref%29))
  (bind _asweapon_wooden_sword (Utilities|Casting|CastToWeapon_WoodenSword OtherActor))
  (bind _asmale_modular_character (Utilities|Casting|CastToMale_ModularCharacter (Game|GetPlayerCharacter 0)))
  (if (Variables|/Game/Flyff-Character/Modular/Male/Male_ModularCharacter.Male_ModularCharacter_C|GetIsAttacking _asmale_modular_character)
    (if (Variables|Default|GetCanBeHitWithMelee)
      (Development|PrintString "SwordHit")
      (bind _returnvalue (Effects|SpawnEmitteratLocation "/Game/SFX/Stylized_FX/Particles/P_Hit.P_Hit" (Transformation|GetActorLocation _asweapon_wooden_sword)))
      (Utilities|FlowControl|Delay 0.01)
      (Components|Activation|Deactivate _returnvalue)
      (Variables|Default|SetHealth (- (Variables|Default|GetHealth) 0.25))
      (if (<= (Variables|Default|GetHealth) 0.0)
        (CallFunction|Death)
        (Actor|DestroyActor)
        (else
          (Variables|Default|SetCanBeHitWithMelee false)
          (Utilities|FlowControl|Delay 0.5)
          (Variables|Default|SetCanBeHitWithMelee true))))))

(event EventBeginPlay)

(event Collision|EventActorBeginOverlap
  (params (OtherActor :type Actor%20Object%20Reference))
  (bind _asmagic_projectile (Utilities|Casting|CastToMagicProjectile OtherActor))
  (Effects|SpawnEmitteratLocation "/Game/SFX/StylizedFX_2/ParticleSystems/P_Explosion_1.P_Explosion_1" (Transformation|GetActorLocation _asmagic_projectile))
  (bind _output_get (Variables|Default|SetHealth (- (Variables|Default|GetHealth) 0.25)))
  (if (<= _output_get 0.0)
    (CallFunction|Death)
    (Actor|DestroyActor _asmagic_projectile)
    (else
      (Actor|DestroyActor _asmagic_projectile))))

(event EventTick
  (params (DeltaSeconds :type Float%20%28single-precision%29))
  (Utilities|FlowControl|Delay 1e+01)
  (if (not (Variables|Default|GetIsMoving))
    (Variables|Default|SetIsMoving true)
    (AI|AIMoveTo self (.RandomLocation (AI|Navigation|GetRandomReachablePointinRadius (Transformation|GetActorLocation) 1e+03 0 0)) 0 5.0 false
      (:OnSuccess
        _)
      (:OnFail
        _))
    (Variables|Default|SetIsMoving false)))

(fn ConstructionScript)

(fn TakeDamage
  (Effects|SpawnEmitteratLocation "/Game/SFX/Stylized_FX/Particles/P_Explosion.P_Explosion" (Transformation|GetActorLocation)))

(fn Death
  (Game|SpawnActorfromClass "/Game/Flyff-Character/Blueprints/LootPickup.LootPickup_C" (Math|Transform|MakeTransform (Transformation|GetSocketLocation (Variables|Character|GetMesh) "foot_r")) "Undefined" 0 0)
  (bind _asthird_person_game_mode (Utilities|Casting|CastToThirdPersonGameMode (Game|GetGameMode)))
  (bind _output_get (Variables|/Game/ThirdPersonBP/Blueprints/ThirdPersonGameMode.ThirdPersonGameMode_C|SetExperience _asthird_person_game_mode (+ (Variables|/Game/ThirdPersonBP/Blueprints/ThirdPersonGameMode.ThirdPersonGameMode_C|GetExperience _asthird_person_game_mode) 1)))
  (if (>= _output_get (Variables|/Game/ThirdPersonBP/Blueprints/ThirdPersonGameMode.ThirdPersonGameMode_C|GetMaxExperience _asthird_person_game_mode))
    (Variables|/Game/ThirdPersonBP/Blueprints/ThirdPersonGameMode.ThirdPersonGameMode_C|SetLevel _asthird_person_game_mode (+ (Variables|/Game/ThirdPersonBP/Blueprints/ThirdPersonGameMode.ThirdPersonGameMode_C|GetLevel _asthird_person_game_mode) 1))
    (Variables|/Game/ThirdPersonBP/Blueprints/ThirdPersonGameMode.ThirdPersonGameMode_C|SetExperience _asthird_person_game_mode 0)
    (Variables|/Game/ThirdPersonBP/Blueprints/ThirdPersonGameMode.ThirdPersonGameMode_C|SetMaxExperience _asthird_person_game_mode (Variables|/Game/ThirdPersonBP/Blueprints/ThirdPersonGameMode.ThirdPersonGameMode_C|GetMaxExperience _asthird_person_game_mode)))
  (bind _asthird_person_game_mode_2 (Utilities|Casting|CastToThirdPersonGameMode (Game|GetGameMode)))
  (Default|UpdateNumbers _asthird_person_game_mode_2)
  (Actor|DestroyActor))